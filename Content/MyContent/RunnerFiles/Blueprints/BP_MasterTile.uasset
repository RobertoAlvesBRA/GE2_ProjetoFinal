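; Base floor tile for a three-lane endless runner that fills itself with random obstacles and pickups on BeginPlay.
; Each lane rolls separately for pines, boxes, coins or rarer items, with the middle lane using its own table.
; When the player overlaps its Box, it requests the next tile from the GameMode, adds points and raises clamped walk speed.
; Only above a speed threshold does it activate the character's Niagara effect and destroy itself after a delay.
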(event OnComponentBeginOverlap(Box)
  (params (OverlappedComponent :type Primitive%20Component%20Object%20Reference) (OtherActor :type Actor%20Object%20Reference) (OtherComp :type Primitive%20Component%20Object%20Reference) (OtherBodyIndex :type Integer) (bFromSweep :type Boolean) (SweepResult :type Hit%20Result%20Structure%20%28by%20ref%29))
  (Utilities|Casting|CastToThirdPersonCharacter OtherActor)
  (bind _asthird_person_game_mode (Utilities|Casting|CastToThirdPersonGameMode (Game|GetGameMode)))
  (Default|SpawnTile _asthird_person_game_mode)
  (bind _asthird_person_game_mode_2 (Utilities|Casting|CastToThirdPersonGameMode (Game|GetGameMode)))
  (Variables|/Game/ThirdPersonBP/Blueprints/ThirdPersonGameMode.ThirdPersonGameMode_C|SetCurrentPoints _asthird_person_game_mode_2 (+ (Variables|/Game/ThirdPersonBP/Blueprints/ThirdPersonGameMode.ThirdPersonGameMode_C|GetCurrentPoints _asthird_person_game_mode_2) (* (Variables|/Game/ThirdPersonBP/Blueprints/ThirdPersonGameMode.ThirdPersonGameMode_C|GetPointsMultiplier _asthird_person_game_mode_2) 1)))
  (bind _asthird_person_character (Utilities|Casting|CastToThirdPersonCharacter (Game|GetPlayerCharacter 0)))
  (Variables|/Script/Engine.CharacterMovementComponent|SetMaxWalkSpeed (Variables|/Script/Engine.Character|GetCharacterMovement _asthird_person_character) (Math|Float|Clamp(Float) (* (Variables|/Script/Engine.CharacterMovementComponent|GetMaxWalkSpeed (Variables|/Script/Engine.Character|GetCharacterMovement _asthird_person_character)) 1.1) 6e+02 1.8e+03))
  (if (>= (* (Variables|/Script/Engine.CharacterMovementComponent|GetMaxWalkSpeed (Variables|/Script/Engine.Character|GetCharacterMovement _asthird_person_character)) 1.1) 1.5e+03)
    (Components|Activation|Activate (Variables|/Game/ThirdPersonBP/Blueprints/ThirdPersonCharacter.ThirdPersonCharacter_C|GetNiagara _asthird_person_character) false)
    (Utilities|FlowControl|Delay 0.5)
    (Actor|DestroyActor)))

(event Custom|teste)

(event EventBeginPlay
  (CallFunction|SpawnObstacles))

(fn ConstructionScript)

(fn SpawnObstacles
  (bind _lane1 (Variables|Default|GetLane1))
  (bind _lane0 (Variables|Default|GetLane0))
  (bind _lane2 (Variables|Default|GetLane2))
  (bind _returnvalue (Transformation|GetWorldTransform _lane0))
  (bind _returnvalue_2 (Transformation|GetWorldTransform _lane2))
  (bind _returnvalue_3 (Transformation|GetWorldTransform _lane1))
  (Utilities|FlowControl|Sequence
    (:then_0
      (switch int (Math|Random|RandomIntegerinRange 0 6)
        (:1
          (Game|SpawnActorfromClass "/Game/MyContent/RunnerFiles/Blueprints/BP_Obstacle_Pine.BP_Obstacle_Pine_C" _returnvalue "Undefined" 0 0))
        (:2
          (if (== (Math|Random|RandomIntegerinRange 0 5) 3)
            (Game|SpawnActorfromClass "/Game/MyContent/RunnerFiles/Blueprints/BP_Pickup_Ima.BP_Pickup_Ima_C" _returnvalue "Undefined" 0 0)))
        (:3
          (if (Math|Random|RandomBool)
            (Game|SpawnActorfromClass "/Game/MyContent/RunnerFiles/Blueprints/BP_Obstacle_Box.BP_Obstacle_Box_C" _returnvalue "Undefined" 0 0)))
        (:4
          (Game|SpawnActorfromClass "/Game/MyContent/RunnerFiles/Blueprints/BP_Pickup_Coin.BP_Pickup_Coin_C" _returnvalue "Undefined" 0 0))))
    (:then_1
      (switch int (Math|Random|RandomIntegerinRange 0 6)
        (:1
          (Game|SpawnActorfromClass "/Game/MyContent/RunnerFiles/Blueprints/BP_Obstacle_Pine.BP_Obstacle_Pine_C" _returnvalue_3 "Undefined" 0 0))
        (:2
          (switch int (Math|Random|RandomIntegerinRange 0 5)
            (:0
              (Game|SpawnActorfromClass "/Game/MyContent/RunnerFiles/Blueprints/BP_Obstacle_Box.BP_Obstacle_Box_C" _returnvalue_3 "Undefined" 0 0))
            (:5
              (Game|SpawnActorfromClass "/Game/MyContent/CamaElastica.CamaElastica_C" _returnvalue_3 "Undefined" 0 0))))
        (:4
          (Game|SpawnActorfromClass "/Game/MyContent/RunnerFiles/Blueprints/BP_Pickup_Coin.BP_Pickup_Coin_C" _returnvalue_3 "Undefined" 0 0))))
    (:then_2
      (switch int (Math|Random|RandomIntegerinRange 0 6)
        (:1
          (Game|SpawnActorfromClass "/Game/MyContent/RunnerFiles/Blueprints/BP_Obstacle_Pine.BP_Obstacle_Pine_C" _returnvalue_2 "Undefined" 0 0))
        (:2
          (if (== (Math|Random|RandomIntegerinRange 0 5) 3)
            (Game|SpawnActorfromClass "/Game/MyContent/RunnerFiles/Blueprints/BP_Pickup_Ima.BP_Pickup_Ima_C" _returnvalue_2 "Undefined" 0 0)))
        (:3
          (if (Math|Random|RandomBool)
            (Game|SpawnActorfromClass "/Game/MyContent/RunnerFiles/Blueprints/BP_Obstacle_Box.BP_Obstacle_Box_C" _returnvalue_2 "Undefined" 0 0)))
        (:4
          (Game|SpawnActorfromClass "/Game/MyContent/RunnerFiles/Blueprints/BP_Pickup_Coin.BP_Pickup_Coin_C" _returnvalue_2 "Undefined" 0 0))))))